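; BP_Generator spawns and clears a two-dimensional grid of BP_Cell actors for procedural generation.
; GenerateLine loops over the truncated Size dimensions, placing cells at CellSize spacing on a fixed elevated height and tracking each in AllCell.
; StarDestroyer destroys every tracked cell and empties the array.
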(event Custom|GenerateLine
  (bind _size (Variables|Default|GetSize))
  (bind (_x _y) (Math|Vector2D|BreakVector2D _size))
  (for _index (range 0 (- (Math|Float|Truncate _x) 1))
    (for _index_2 (range 0 (- (Math|Float|Truncate _y) 1))
      (bind _returnvalue (Game|SpawnActorfromClass "/Game/Blueprint/Procedural/BP_Cell.BP_Cell_C" (Math|Transform|MakeTransform (Math|Vector|MakeVector (* _index_2 (Variables|Default|GetCellSize)) (* _index (Variables|Default|GetCellSize)) 2e+03) "0, 0, 0" "1.000000,1.000000,1.000000") "Undefined" "MultiplyWithRoot" 0 0))
      (Utilities|Array|AddUnique (Variables|Default|GetAll_Cell) _returnvalue))))

(event Custom|StarDestroyer
  (bind _all_cell (Variables|Default|GetAll_Cell))
  (for _array_element _all_cell
    (Actor|DestroyActor _array_element))
  (Utilities|Array|Clear _all_cell))

(fn ConstructionScript)