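; BP_BonusZoneCritique is a pickup that grants the player a critical-zone bonus tier set by its EnumZone value.
; On BeginPlay, EnumZone selects one of five bonus materials for the static mesh so each tier looks different.
; When the player character overlaps it, the pickup passes EnumZone to BP_Character's BonusZoneCritique, then destroys itself.
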(event OnComponentBeginOverlap()
  (params (OverlappedComponent :type Primitive%20Component%20Object%20Reference) (OtherActor :type Actor%20Object%20Reference) (OtherComp :type Primitive%20Component%20Object%20Reference) (OtherBodyIndex :type Integer) (bFromSweep :type Boolean) (SweepResult :type Hit%20Result%20Structure%20%28by%20ref%29))
  (bind _returnvalue (Game|GetPlayerCharacter 0))
  (if (== OtherActor _returnvalue)
    (bind _asbp_character (Utilities|Casting|CastToBP_Character _returnvalue))
    (Default|BonusZoneCritique _asbp_character (Variables|Default|GetEnum_zone))
    (Actor|DestroyActor)))

(event EventBeginPlay
  (switch Utilities|FlowControl|Switch|SwitchonEnum_BonusZoneCritique (Variables|Default|GetEnum_zone)
    (:NewEnumerator0
      (Rendering|Material|SetMaterial (Variables|Default|GetStaticMesh) 0 "/Game/Material/Bonus/Bonus1.Bonus1"))
    (:NewEnumerator1
      (Rendering|Material|SetMaterial (Variables|Default|GetStaticMesh) 0 "/Game/Material/Bonus/Bonus2.Bonus2"))
    (:NewEnumerator2
      (Rendering|Material|SetMaterial (Variables|Default|GetStaticMesh) 0 "/Game/Material/Bonus/Bonus3.Bonus3"))
    (:NewEnumerator3
      (Rendering|Material|SetMaterial (Variables|Default|GetStaticMesh) 0 "/Game/Material/Bonus/Bonus4.Bonus4"))
    (:NewEnumerator4
      (Rendering|Material|SetMaterial (Variables|Default|GetStaticMesh) 0 "/Game/Material/Bonus/Bonus5.Bonus5"))))

(fn ConstructionScript)