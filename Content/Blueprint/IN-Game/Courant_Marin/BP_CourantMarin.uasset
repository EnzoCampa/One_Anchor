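; BP_CourantMarin is a sea current trigger that displaces the player character along what its naming suggests is Y.
; When the player overlaps its Box while BPeutSeDeplacer is true, a half-second looping timer starts.
; On its first tick, the timer calls YDeplacement on the cached BP_Character with itself as argument, clears BPeutSeDeplacer and cancels itself.
; Nothing here resets the flag, so the current works as a delayed one-shot.
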(event OnComponentBeginOverlap(Box)
  (params (OverlappedComponent :type Primitive%20Component%20Object%20Reference) (OtherActor :type Actor%20Object%20Reference) (OtherComp :type Primitive%20Component%20Object%20Reference) (OtherBodyIndex :type Integer) (bFromSweep :type Boolean) (SweepResult :type Hit%20Result%20Structure%20%28by%20ref%29))
  (if (== OtherActor (Game|GetPlayerCharacter 0))
    (if (Variables|Default|GetBPeutSeDeplacer)
      (bind _returnvalue (Utilities|Time|SetTimerbyEvent (delegate Custom|deplacemnt%20Y%20courrant%20marin) 0.5 true)))))

(event Custom|deplacemnt%20Y%20courrant%20marin
  (Default|YDeplacement (Variables|Default|GetAs%20BP%20Character) self)
  (Variables|Default|SetBPeutSeDeplacer false)
  (Utilities|Time|ClearandInvalidateTimerbyHandle (stale OnComponentBeginOverlap(Box) _returnvalue)))

(event EventBeginPlay
  (bind _asbp_character (Utilities|Casting|CastToBP_Character (Game|GetPlayerCharacter 0)))
  (Variables|Default|SetAs%20BP%20Character _asbp_character))

(fn ConstructionScript)