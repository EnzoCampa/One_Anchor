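; GI_Games is the Game Instance that handles level win and loss screens and owns the save game.
; LooseLevel and WinLevel each show their HUD widget, pause the game and have PC_Game set the mouse cursor.
; Init loads the SG_SaveGame slot or creates a new save object, then starts a looping timer that autosaves it every few seconds.
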(event Custom|Win%20Level
  (bind _returnvalue (UserInterface|CreateWidget "/Game/UserInterface/HUD_Win.HUD_Win_C"))
  (UserInterface|Viewport|AddtoViewport _returnvalue 0)
  (Game|SetGamePaused true)
  (bind _aspc_game (Utilities|Casting|CastToPC_Game (Game|GetPlayerController 0)))
  (Default|SetMouseCursor _aspc_game))

(event Custom|SaveGame
  (SaveGame|SaveGametoSlot (Variables|Default|GetTest%20Save) (Variables|Default|GetTest%20Slot%20Name)))

(event Custom|Loose%20Level
  ;[0.15 0.15 0.15 0.5] Ici je cast l'HUD restart quand je touche le sol et je pause le jeu. Ensuite je récupère mon Player Controller pour activer la souris
  (bind _returnvalue (UserInterface|CreateWidget "/Game/UserInterface/HUD_Restart.HUD_Restart_C"))
  (UserInterface|Viewport|AddtoViewport _returnvalue 0)
  (Game|SetGamePaused true)
  (bind _aspc_game (Utilities|Casting|CastToPC_Game (Game|GetPlayerController 0)))
  (Default|SetMouseCursor _aspc_game))

(event EventInit
  (bind _returnvalue (SaveGame|DoesSaveGameExist (Variables|Default|GetTest%20Slot%20Name)))
  (if _returnvalue
    (bind _returnvalue_2 (SaveGame|LoadGamefromSlot (Variables|Default|GetTest%20Slot%20Name)))
    (Variables|Default|SetTest%20Save (.AsSG%20Save%20Game (Utilities|Casting|CastToSG_SaveGame _returnvalue_2)))
    (else
      (bind _returnvalue_3 (SaveGame|CreateSaveGameObject "/Game/Blueprint/IN-Game/SG_SaveGame.SG_SaveGame_C"))
      (Variables|Default|SetTest%20Save _returnvalue_3)))
  (Utilities|Time|SetTimerbyEvent (delegate Custom|SaveGame) 5.0 true))