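; Game mode that runs the start-of-game countdown before the player character can move.
; A looping half-second timer set on BeginPlay polls until the player character is valid, then a DoOnce lets the sequence run a single time.
; It shows the countdown HUD widget, waits about three seconds, then sets the character's BEnMouvement flag to true.
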(event Custom|StopCharacter
  (bind _returnvalue (Game|GetPlayerCharacter 0))
  ;[0.15 0.15 0.15 0.5] Je vérifie d'abord que mon character existe
  (Utilities|IsValid _returnvalue
    (:Is%20Valid
      ;[0.15 0.15 0.15 0.5] Si il existe je bloque son mouvement
      (Utilities|FlowControl|DoOnce false
        (:Completed
          (bind _asbp_character (Utilities|Casting|CastToBP_Character _returnvalue))
          ;[0.15 0.15 0.15 0.5] Ensuite je lance mon HUD puis je réactive 3s plus tard les déplacements
          (bind _returnvalue_2 (UserInterface|CreateWidget "/Game/UserInterface/HUD_CooldwonBeforeStart.HUD_CooldwonBeforeStart_C"))
          (UserInterface|Viewport|AddtoViewport _returnvalue_2 0)
          (Default|HUDStarter _returnvalue_2)
          (Utilities|FlowControl|Delay 3.2)
          (Variables|/Game/Blueprint/IN-Game/Character/BP_Character.BP_Character_C|SetBEnMouvement _asbp_character true))))))

(event EventBeginPlay
  ;[0.15 0.15 0.15 0.5] Je crée un timer
  (Utilities|Time|SetTimerbyEvent (delegate Custom|StopCharacter) 0.5 true))

(fn ConstructionScript)