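; BP_SasDeLevel is an airlock trigger between or at the end of levels that checks the player's landing speed.
; On first overlap it zeroes CurrentSpeed and kills the character if GravitySpeed is at or below SpeedMax.
; Otherwise EnumSas either ends the level or starts refueling: fuel use is blocked and a looping timer event tops fuel up to FuelVarInit, then plays the opening timeline.
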(event OnComponentBeginOverlap(Box)
  (params (OverlappedComponent :type Primitive%20Component%20Object%20Reference) (OtherActor :type Actor%20Object%20Reference) (OtherComp :type Primitive%20Component%20Object%20Reference) (OtherBodyIndex :type Integer) (bFromSweep :type Boolean) (SweepResult :type Hit%20Result%20Structure%20%28by%20ref%29))
  (bind _returnvalue (Game|GetPlayerCharacter 0))
  (if (== OtherActor _returnvalue)
    (bind _asbp_character (Utilities|Casting|CastToBP_Character _returnvalue))
    (Variables|Default|SetAs%20BP%20Character _asbp_character)
    (CallFunction|VItesse?)))

(event Custom|VItesse%20?
  (bind _as_bp_character (Variables|Default|GetAs%20BP%20Character))
  (bind _as_bp_character_2 (Variables|Default|GetAs%20BP%20Character))
  (Utilities|FlowControl|DoOnce false
    (:Completed
      (Variables|/Game/Blueprint/IN-Game/Character/BP_Character.BP_Character_C|SetCurrentSpeed (Variables|Default|GetAs%20BP%20Character) 0.0)
      (if (<= (Variables|/Game/Blueprint/IN-Game/Character/BP_Character.BP_Character_C|GetGravitySpeed _as_bp_character) (Variables|/Game/Blueprint/IN-Game/Character/BP_Character.BP_Character_C|GetSpeed%20Max _as_bp_character))
        (Default|Mort _as_bp_character_2)
        (else
          (switch Utilities|FlowControl|Switch|SwitchonEnum_SasDeLevel (Variables|Default|Getenum_sas)
            (:NewEnumerator0
              (Default|FinDeLevel _as_bp_character_2))
            (:NewEnumerator1
              (CallFunction|RechargementFuel))))))))

(event Custom|Ouverture%20du%20sas
  (Timeline|Timeline%20Sas%20FIn%20De%20Zone Play))

(event Custom|RechargementFuel
  (Variables|/Game/Blueprint/IN-Game/Character/BP_Character.BP_Character_C|SetBBlockFuelUse (Variables|Default|GetAs%20BP%20Character) true)
  (Utilities|Time|SetTimerbyEvent (delegate Custom|Reload) 0.0 true))

(event Custom|Reload
  (bind _as_bp_character (Variables|Default|GetAs%20BP%20Character))
  (bind _as_bp_character_2 (Variables|Default|GetAs%20BP%20Character))
  (while (> (Variables|/Game/Blueprint/IN-Game/Character/BP_Character.BP_Character_C|GetFuel%20Var%20Init _as_bp_character) (Variables|/Game/Blueprint/IN-Game/Character/BP_Character.BP_Character_C|GetFuelVar _as_bp_character))
    (Variables|/Game/Blueprint/IN-Game/Character/BP_Character.BP_Character_C|SetFuelVar _as_bp_character_2 (+ (Variables|/Game/Blueprint/IN-Game/Character/BP_Character.BP_Character_C|GetFuelVar _as_bp_character_2) 2.0)))
  (CallFunction|OuvertureDuSas))

(fn ConstructionScript)