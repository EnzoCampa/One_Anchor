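; BP_ZoneGravite is a trigger zone that modifies the player character's gravity while they are inside it.
; Box overlap events respond only to player 0 and cast it to BP_Character.
; Entering passes the zone's random float min and max to the character's ZoneChangementGravité, and leaving calls StopGravityModyfying, so the gravity logic itself lives in the character.
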(event OnComponentBeginOverlap(Box)
  (params (OverlappedComponent :type Primitive%20Component%20Object%20Reference) (OtherActor :type Actor%20Object%20Reference) (OtherComp :type Primitive%20Component%20Object%20Reference) (OtherBodyIndex :type Integer) (bFromSweep :type Boolean) (SweepResult :type Hit%20Result%20Structure%20%28by%20ref%29))
  (bind _returnvalue (Game|GetPlayerCharacter 0))
  (if (== OtherActor _returnvalue)
    (bind _asbp_character (Utilities|Casting|CastToBP_Character _returnvalue))
    (Default|ZoneChangementGravité _asbp_character (Variables|Default|GetRandom%20Float%20Min) (Variables|Default|GetRandom%20Float%20Max))))

(event OnComponentEndOverlap(Box)
  (params (OverlappedComponent :type Primitive%20Component%20Object%20Reference) (OtherActor :type Actor%20Object%20Reference) (OtherComp :type Primitive%20Component%20Object%20Reference) (OtherBodyIndex :type Integer))
  (bind _returnvalue (Game|GetPlayerCharacter 0))
  (if (== OtherActor _returnvalue)
    (bind _asbp_character (Utilities|Casting|CastToBP_Character _returnvalue))
    (Default|StopGravityModyfying _asbp_character)))

(fn ConstructionScript)