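; BP_Sas is an airlock with two sliding doors that cycle endlessly once triggered and can kill the player.
; The player's first TriggerZone overlap turns detector cubes from green to orange, then starts the cycle after a delay.
; One Timeline lerps both doors by SlideDistance, alternating play and reverse through BIsOpen with a pause between moves.
; Door collision boxes call Mort on BP_Character, though the right box compares OtherComp instead of OtherActor.
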(event OnComponentBeginOverlap(TriggerZone)
  (params (OverlappedComponent :type Primitive%20Component%20Object%20Reference) (OtherActor :type Actor%20Object%20Reference) (OtherComp :type Primitive%20Component%20Object%20Reference) (OtherBodyIndex :type Integer) (bFromSweep :type Boolean) (SweepResult :type Hit%20Result%20Structure%20%28by%20ref%29))
  ;[0.15 0.15 0.15 0.5] Récupérer le character pour déclanchement du sas
  (Utilities|IsValid OtherActor
    (:Is%20Valid
      (if (== OtherActor (Game|GetPlayerCharacter 0))
        (Utilities|FlowControl|DoOnce false
          (:Completed
            (CallFunction|ChangementDeCouleur)
            (Utilities|FlowControl|Delay (Variables|Fermeture|GetOffsetBeforeLaunching))
            (CallFunction|FermetureSas)))))))

(event OnComponentBeginOverlap(BoxCollisionRightDoor)
  (params (OverlappedComponent :type Primitive%20Component%20Object%20Reference) (OtherActor :type Actor%20Object%20Reference) (OtherComp :type Primitive%20Component%20Object%20Reference) (OtherBodyIndex :type Integer) (bFromSweep :type Boolean) (SweepResult :type Hit%20Result%20Structure%20%28by%20ref%29))
  (bind _returnvalue (Game|GetPlayerCharacter 0))
  ;[0.15 0.15 0.15 0.5] Vérification si le PC est bien l'entité touché, si oui on déclanche la mort
  (if (== OtherComp _returnvalue)
    (bind _asbp_character (Utilities|Casting|CastToBP_Character _returnvalue))
    (Default|Mort _asbp_character)))

(event OnComponentBeginOverlap(BoxCollisionLeftDoor)
  (params (OverlappedComponent :type Primitive%20Component%20Object%20Reference) (OtherActor :type Actor%20Object%20Reference) (OtherComp :type Primitive%20Component%20Object%20Reference) (OtherBodyIndex :type Integer) (bFromSweep :type Boolean) (SweepResult :type Hit%20Result%20Structure%20%28by%20ref%29))
  (bind _returnvalue (Game|GetPlayerCharacter 0))
  ;[0.15 0.15 0.15 0.5] Vérification si le PC est bien l'entité touché, si oui on déclanche la mort
  (if (== _returnvalue OtherActor)
    (bind _asbp_character (Utilities|Casting|CastToBP_Character _returnvalue))
    (Default|Mort _asbp_character)))

(event Custom|Fermeture%20sas
  (Utilities|FlowControl|Delay (Variables|Fermeture|GetDelayBeforeWorking))
  ;[0.15 0.15 0.15 0.5] Déplacement et animation des portes via la timeline et on lerp les positions des portes
  (CallFunction|Revert)
  (bind _newtrack_0 (Timeline|Timeline Play)
    (:Update
      (Transformation|SetRelativeLocation (Variables|Default|GetLeftDoor) (Math|Vector|Lerp(Vector) (Variables|Fermeture|GetLeftClosePos) (Variables|Fermeture|GetLeftOpenPose) _newtrack_0) false false)
      (Transformation|SetRelativeLocation (Variables|Default|GetRightDoor) (Math|Vector|Lerp(Vector) (Variables|Fermeture|GetRightClosePos) (Variables|Fermeture|GetRightOpenPose) _newtrack_0) false false))
    (:Finished
      (if (Variables|Default|GetBIsOpen)
        (Variables|Default|SetBIsOpen false)
        (CallFunction|FermetureSas)
        (else
          (Variables|Default|SetBIsOpen true)
          (CallFunction|ReverseTimeline))))))

(event Custom|Changement%20de%20couleur
  (Utilities|FlowControl|DoOnce false
    (:Completed
      (Rendering|Material|SetMaterial (Variables|Default|GetCube) 0 "/Game/Material/Mat_SasDetecteurColorOrange.Mat_SasDetecteurColorOrange"))))

(event Custom|Reverse%20Timeline
  ;[0.15 0.15 0.15 0.5] Déplacement et animation des portes via la timeline et on lerp les positions des portes
  (Utilities|FlowControl|Delay (Variables|Fermeture|GetDelayBeforeWorking))
  (CallFunction|Revert)
  (bind _newtrack_0 (Timeline|Timeline ReverseFromEnd)
    (:Update
      (Transformation|SetRelativeLocation (Variables|Default|GetLeftDoor) (Math|Vector|Lerp(Vector) (Variables|Fermeture|GetLeftClosePos) (Variables|Fermeture|GetLeftOpenPose) _newtrack_0) false false)
      (Transformation|SetRelativeLocation (Variables|Default|GetRightDoor) (Math|Vector|Lerp(Vector) (Variables|Fermeture|GetRightClosePos) (Variables|Fermeture|GetRightOpenPose) _newtrack_0) false false))
    (:Finished
      (if (Variables|Default|GetBIsOpen)
        (Variables|Default|SetBIsOpen false)
        (CallFunction|FermetureSas)
        (else
          (Variables|Default|SetBIsOpen true)
          (CallFunction|ReverseTimeline))))))

(event EventBeginPlay
  (Variables|Fermeture|SetLeftClosePos (Variables|/Script/Engine.SceneComponent|GetRelativeLocation (Variables|Default|GetLeftDoor)))
  (Variables|Fermeture|SetRightClosePos (Variables|/Script/Engine.SceneComponent|GetRelativeLocation (Variables|Default|GetRightDoor)))
  (Variables|Fermeture|SetRightOpenPose (- (Variables|/Script/Engine.SceneComponent|GetRelativeLocation (Variables|Default|GetRightDoor)) (Math|Vector|MakeVector 0.0 (Variables|Fermeture|GetSlideDistance) 0.0)))
  (Variables|Fermeture|SetLeftOpenPose (+ (Variables|/Script/Engine.SceneComponent|GetRelativeLocation (Variables|Default|GetLeftDoor)) (Math|Vector|MakeVector 0.0 (Variables|Fermeture|GetSlideDistance) 0.0)))
  (Rendering|Material|SetMaterial (Variables|Default|GetCube) 0 "/Game/Material/Mat_SasDetecteurColorGreen.Mat_SasDetecteurColorGreen"))

(fn ConstructionScript)

(fn Revert
  (bind _right_arrow (Variables|Default|GetRight%20Arrow))
  (bind _left_arrow (Variables|Default|GetLeft%20Arrow))
  (bind _right_arrow_2 (Variables|Default|GetRight%20Arrow))
  (bind _left_arrow_2 (Variables|Default|GetLeft%20Arrow))
  (bind _relativerotation (Variables|/Script/Engine.SceneComponent|GetRelativeRotation _right_arrow))
  (bind _relativerotation_2 (Variables|/Script/Engine.SceneComponent|GetRelativeRotation _left_arrow))
  (bind _relativerotation_3 (Variables|/Script/Engine.SceneComponent|GetRelativeRotation _left_arrow_2))
  (bind _relativerotation_4 (Variables|/Script/Engine.SceneComponent|GetRelativeRotation _right_arrow_2))
  (if (Variables|Default|GetBIsOpen)
    (Transformation|SetRelativeRotation (Variables|Default|GetRight%20Arrow1) (Math|Rotator|MakeRotator (.roll _relativerotation) 1.8e+02 (.yaw _relativerotation)) false false)
    (Transformation|SetRelativeRotation (Variables|Default|GetLeft%20Arrow1) (Math|Rotator|MakeRotator (.roll _relativerotation_2) 1.8e+02 (.yaw _relativerotation_2)) false false)
    (else
      (Transformation|SetRelativeRotation (Variables|Default|GetRight%20Arrow1) (Math|Rotator|MakeRotator (.roll _relativerotation_4) 1.8e+02 (.yaw _relativerotation_4)) false false)
      (Transformation|SetRelativeRotation (Variables|Default|GetLeft%20Arrow1) (Math|Rotator|MakeRotator (.roll _relativerotation_3) 1.8e+02 (.yaw _relativerotation_3)) false false)))
  (return))