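; BP_Poissong is an enemy that chases the player and kills them on contact, with capsule physics and gravity off.
; Entering Box1 starts a one-shot-gated looping timer that moves the Poissong component toward the player at constant speed, facing them.
; Leaving Box1 clears the timer and destroys the actor after a short delay.
; Overlapping Box calls Mort on BP_Character to trigger death.
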(event OnComponentEndOverlap(Box1)
  (params (OverlappedComponent :type Primitive%20Component%20Object%20Reference) (OtherActor :type Actor%20Object%20Reference) (OtherComp :type Primitive%20Component%20Object%20Reference) (OtherBodyIndex :type Integer))
  ;[0.15 0.15 0.15 0.5] Quand le character sort je désactive le timer
  (if (== OtherActor (Game|GetPlayerCharacter 0))
    (Utilities|Time|ClearandInvalidateTimerbyHandle (Variables|Default|GetTimerHandle))
    (Utilities|FlowControl|Delay 0.2)
    (Actor|DestroyActor)))

(event OnComponentBeginOverlap(Box)
  (params (OverlappedComponent :type Primitive%20Component%20Object%20Reference) (OtherActor :type Actor%20Object%20Reference) (OtherComp :type Primitive%20Component%20Object%20Reference) (OtherBodyIndex :type Integer) (bFromSweep :type Boolean) (SweepResult :type Hit%20Result%20Structure%20%28by%20ref%29))
  ;[0.15 0.15 0.15 0.5] Si le projectile touche le character alors trigger mort dans bp_character
  (if (== OtherActor (Game|GetPlayerCharacter 0))
    (bind _asbp_character (Utilities|Casting|CastToBP_Character (Game|GetPlayerCharacter 0)))
    (Default|Mort _asbp_character)))

(event OnComponentBeginOverlap(Box1)
  (params (OverlappedComponent :type Primitive%20Component%20Object%20Reference) (OtherActor :type Actor%20Object%20Reference) (OtherComp :type Primitive%20Component%20Object%20Reference) (OtherBodyIndex :type Integer) (bFromSweep :type Boolean) (SweepResult :type Hit%20Result%20Structure%20%28by%20ref%29))
  ;[0.15 0.15 0.15 0.5] On component hit je lance le timer
  (if (== OtherActor (Game|GetPlayerCharacter 0))
    (Variables|Default|SetCharacter OtherActor)
    (Utilities|FlowControl|DoOnce false
      (:Completed
        (bind _returnvalue (Utilities|Time|SetTimerbyEvent (delegate Custom|DéplacementDeLacteur) 0.016 true))
        (Variables|Default|SetTimerHandle _returnvalue)))))

(event Custom|DéplacementDeLacteur
  (bind _character (Variables|Default|GetCharacter))
  (bind _poissong (Variables|Default|GetPoissong))
  (bind _returnvalue (Transformation|GetActorLocation _character))
  (bind _returnvalue_2 (Transformation|GetWorldLocation _poissong))
  (bind _returnvalue_3 (Math|Rotator|FindLookatRotation _returnvalue_2 _returnvalue))
  ;[0.15 0.15 0.15 0.5] Je déplace mon character en fonction des positionements
  (Transformation|SetWorldLocation (Variables|Default|GetPoissong) (Math|Interpolation|VInterptoConstant (Transformation|GetWorldLocation (Variables|Default|GetPoissong)) (Transformation|GetActorLocation (Variables|Default|GetCharacter)) (Variables|Default|GetTime) (Variables|Default|GetV%20Interp%20Speed)) false false)
  (Transformation|SetRelativeRotation (Variables|Default|GetPoissong) (Math|Rotator|MakeRotator 0.0 (.pitch _returnvalue_3) (.yaw _returnvalue_3)) false false))

(event EventBeginPlay
  (bind _capsulecomponent (Variables|Collision|GetCapsuleComponent))
  ;[0.15 0.15 0.15 0.5] J'étaibli la physique et la gravité a false
  (Physics|SetSimulatePhysics _capsulecomponent false)
  (Physics|SetEnableGravity _capsulecomponent false))

(fn ConstructionScript)