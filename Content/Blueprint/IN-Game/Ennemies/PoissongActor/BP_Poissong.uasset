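; BP_Poissong is a fish enemy that chases the player and kills on contact through the character's Mort.
; Entering Box2 starts a looping timer that interpolates the fish toward the player and turns it to face them.
; CollisionDash interrupts the chase for a timeline-driven velocity dash on the Y/Z plane, then resumes it.
; Box1 and Box2 detach at BeginPlay as fixed world zones; leaving Box1 destroys the fish after a short delay.
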(event OnComponentBeginOverlap(Box2)
  (params (OverlappedComponent :type Primitive%20Component%20Object%20Reference) (OtherActor :type Actor%20Object%20Reference) (OtherComp :type Primitive%20Component%20Object%20Reference) (OtherBodyIndex :type Integer) (bFromSweep :type Boolean) (SweepResult :type Hit%20Result%20Structure%20%28by%20ref%29))
  (bind _asbp_character (Utilities|Casting|CastToBP_Character OtherActor))
  ;[0.15 0.15 0.15 0.5] On component hit je lance le timer
  (Variables|Default|SetAs%20BP%20Character _asbp_character)
  (Utilities|Time|ClearandInvalidateTimerbyHandle (Variables|Default|GetTimeHandle%20Déplacement))
  (Utilities|FlowControl|DoOnce false
    (:Completed
      (bind _returnvalue (Utilities|Time|SetTimerbyEvent (delegate Custom|DéplacementDeLacteur) 0.016667 true))
      (Variables|Default|SetTimerHandle _returnvalue))))

(event OnComponentEndOverlap(Box1)
  (params (OverlappedComponent :type Primitive%20Component%20Object%20Reference) (OtherActor :type Actor%20Object%20Reference) (OtherComp :type Primitive%20Component%20Object%20Reference) (OtherBodyIndex :type Integer))
  ;[0.15 0.15 0.15 0.5] Quand le character sort je désactive le timer
  (if (== OtherActor (Game|GetPlayerCharacter 0))
    (Utilities|Time|ClearandInvalidateTimerbyHandle (Variables|Default|GetTimerHandle))
    (Utilities|FlowControl|Delay 0.2)
    (Actor|DestroyActor)))

(event OnComponentBeginOverlap(Box)
  (params (OverlappedComponent :type Primitive%20Component%20Object%20Reference) (OtherActor :type Actor%20Object%20Reference) (OtherComp :type Primitive%20Component%20Object%20Reference) (OtherBodyIndex :type Integer) (bFromSweep :type Boolean) (SweepResult :type Hit%20Result%20Structure%20%28by%20ref%29))
  ;[0.15 0.15 0.15 0.5] Si le projectile touche le character alors trigger mort dans bp_character
  (if (== OtherActor (Game|GetPlayerCharacter 0))
    (bind _asbp_character (Utilities|Casting|CastToBP_Character (Game|GetPlayerCharacter 0)))
    (Default|Mort _asbp_character)))

(event OnComponentBeginOverlap(CollisionDash)
  (params (OverlappedComponent :type Primitive%20Component%20Object%20Reference) (OtherActor :type Actor%20Object%20Reference) (OtherComp :type Primitive%20Component%20Object%20Reference) (OtherBodyIndex :type Integer) (bFromSweep :type Boolean) (SweepResult :type Hit%20Result%20Structure%20%28by%20ref%29))
  ;[0.15 0.15 0.15 0.5] Trigger Dash
  (if (== OtherActor (Game|GetPlayerCharacter 0))
    (CallFunction|DashEvent)))

(event Custom|DéplacementDeLacteur
  (bind _poissong (Variables|Default|GetPoissong))
  (bind _as_bp_character (Variables|Default|GetAs%20BP%20Character))
  (bind _returnvalue (Transformation|GetActorLocation _as_bp_character))
  (bind _returnvalue_2 (Transformation|GetWorldLocation _poissong))
  (bind _returnvalue_3 (Math|Rotator|FindLookatRotation (Math|Vector|MakeVector 0.0 (.y _returnvalue_2) (.z _returnvalue_2)) (Math|Vector|MakeVector 0.0 (.y _returnvalue) (.z _returnvalue))))
  (bind (_roll _pitch _yaw) (Math|Rotator|BreakRotator _returnvalue_3))
  ;[0.15 0.15 0.15 0.5] Je déplace mon character en fonction des positionements
  (Transformation|SetWorldLocation (Variables|Default|GetPoissong) (Math|Interpolation|VInterpTo (Transformation|GetWorldLocation (Variables|Default|GetPoissong)) (Transformation|GetWorldLocation (Variables|/Script/Engine.Character|GetMesh (Variables|Default|GetAs%20BP%20Character))) (Utilities|Time|GetWorldDeltaSeconds) (Variables|Default|GetV%20Interp%20Speed)) false false)
  (Transformation|SetWorldRotation (Variables|Default|GetPoissong) (Math|Rotator|MakeRotator _roll _pitch _yaw) false false))

(event Custom|DashEvent
  ;[0.15 0.15 0.15 0.5] Dash
  (Utilities|FlowControl|DoOnce false
    (:Completed
      (Variables|Default|SetLast%20character%20position (Transformation|GetWorldLocation (Variables|/Script/Engine.Character|GetMesh (Variables|Default|GetAs%20BP%20Character))))
      (Utilities|Time|ClearandInvalidateTimerbyHandle (Variables|Default|GetTimerHandle))
      (bind _track_dash (Timeline|Timeline%20Dash PlayFromStart)
        (:Update
          (Variables|/Script/Engine.MovementComponent|SetVelocity (Variables|Character|GetCharacterMovement) (Math|Vector|MakeVector 0.0 (.y (* (Math|Vector|GetForwardVector (Variables|Default|GetPoissong)) (* _track_dash (Variables|Default|GetDistance%20Dash)))) (.z (* (Math|Vector|GetForwardVector (Variables|Default|GetPoissong)) (* _track_dash (Variables|Default|GetDistance%20Dash)))))))
        (:Finished
          (Components|Movement|StopMovementImmediately (Variables|Character|GetCharacterMovement))
          (CallFunction|ResetDash)
          (CallFunction|PlayTimer))))))

(event Custom|reset%20dash
  ;[0.15 0.15 0.15 0.5] Dash
  (Utilities|FlowControl|DoOnce false) ; enters at Reset
)

(event Custom|Play%20timer
  ;[0.15 0.15 0.15 0.5] On component hit je lance le timer
  (bind _returnvalue (Utilities|Time|SetTimerbyEvent (delegate Custom|DéplacementDeLacteur) 0.016667 true))
  (Variables|Default|SetTimerHandle _returnvalue))

(event EventBeginPlay
  (bind _capsulecomponent (Variables|Collision|GetCapsuleComponent))
  ;[0.15 0.15 0.15 0.5] J'étaibli la physique et la gravité a false
  (Variables|Default|SetStart%20Pos (Transformation|GetWorldLocation (Variables|Default|GetPoissong)))
  (Utilities|Casting|CastToBP_Character (Game|GetPlayerCharacter 0))
  (Physics|SetSimulatePhysics _capsulecomponent false)
  (Physics|SetEnableGravity _capsulecomponent false)
  (Transformation|DetachFromComponent (Variables|Default|GetBox1) "KeepWorld" "KeepWorld" "KeepWorld" true))

(fn ConstructionScript)