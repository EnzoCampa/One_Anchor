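; BP_Malus is an enemy hazard that temporarily blocks the player character's fuel use.
; Entering the outer Box reveals it as a sphere, then destroys it after DurationDespawn unless the malus has triggered.
; Touching MalusCollider shows the HUD_ZoneCritique widget, clears the mesh and calls BlockFuelUse on BP_Character.
; After DurationMalus, it calls BlockFuelUse again, removes the widget and destroys itself.
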(event OnComponentBeginOverlap(Box)
  (params (OverlappedComponent :type Primitive%20Component%20Object%20Reference) (OtherActor :type Actor%20Object%20Reference) (OtherComp :type Primitive%20Component%20Object%20Reference) (OtherBodyIndex :type Integer) (bFromSweep :type Boolean) (SweepResult :type Hit%20Result%20Structure%20%28by%20ref%29))
  (bind _malus (Variables|Default|GetMalus))
  ;[0.15 0.15 0.15 0.5] Je set le material et son mesh
  (if (== OtherActor (Game|GetPlayerCharacter 0))
    (Components|StaticMesh|SetStaticMesh _malus "/Engine/EngineMeshes/Sphere.Sphere")
    (Rendering|Material|SetMaterial _malus 0 "/Engine/MapTemplates/Materials/BasicAsset01.BasicAsset01")
    ;[0.15 0.15 0.15 0.5] Après un delay je fais despawn le character
    (Utilities|FlowControl|Delay (Variables|Default|GetDuration%20Despawn))
    (if (not (Variables|Default|GetFuelBlocked))
      (Actor|DestroyActor))))

(event OnComponentBeginOverlap(MalusCollider)
  (params (OverlappedComponent :type Primitive%20Component%20Object%20Reference) (OtherActor :type Actor%20Object%20Reference) (OtherComp :type Primitive%20Component%20Object%20Reference) (OtherBodyIndex :type Integer) (bFromSweep :type Boolean) (SweepResult :type Hit%20Result%20Structure%20%28by%20ref%29))
  (bind _returnvalue (Game|GetPlayerCharacter 0))
  (bind _malus (Variables|Default|GetMalus))
  ;[0.15 0.15 0.15 0.5] Bloquer le bouton pendant 1s
  (if (== OtherActor _returnvalue)
    (bind _asbp_character (Utilities|Casting|CastToBP_Character _returnvalue))
    (UserInterface|Viewport|AddtoViewport (Variables|Default|GetHUD%20Zone%20Critique) 0)
    (Variables|Default|SetFuelBlocked true)
    (Default|BlockFuelUse _asbp_character)
    (Components|StaticMesh|SetStaticMesh _malus 0)
    (Rendering|Material|SetMaterial _malus 0 0)
    (Utilities|FlowControl|Delay (Variables|Default|GetDuration%20Malus))
    (Default|BlockFuelUse _asbp_character)
    (Widget|RemovefromParent (Variables|Default|GetHUD%20Zone%20Critique))
    (Actor|DestroyActor)))

(event EventBeginPlay
  ;[0.15 0.15 0.15 0.5] Récupération du HUD
  (bind _returnvalue (UserInterface|CreateWidget "/Game/UserInterface/HUD_ZoneCritique.HUD_ZoneCritique_C"))
  (Variables|Default|SetHUD%20Zone%20Critique _returnvalue))

(fn ConstructionScript)